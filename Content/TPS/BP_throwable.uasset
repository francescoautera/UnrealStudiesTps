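; BP_throwable is a timed throwable for the TPS game that explodes and makes noise AI can hear.
; On BeginPlay it applies its weapon mesh and launches it with the Toss velocity through physics.
; Tick accumulates time until TimeToDestroy, then spawns the hit effect and explosion sound, reports a noise event with player 0 as instigator, and destroys itself.
; The graph applies no damage.
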(event `self.ReceiveBeginPlay`
  (bind _mesh (`self.Mesh`))
  (`StaticMeshComponent.SetStaticMesh` _mesh (`self.WeaponMesh`))
  (`PrimitiveComponent.SetPhysicsLinearVelocity` _mesh (`self.Toss`) false "None"))

(event `self.ReceiveTick`
  (params (DeltaSeconds :type "Float (single-precision)"))
  (bind _returnvalue (`SceneComponent.K2_GetComponentLocation` (`self.Mesh`)))
  (bind _output_get (set `self.ElapsedTime` (+ DeltaSeconds (`self.ElapsedTime`))))
  (if (>= _output_get (`self.TimeToDestroy`))
    (`GameplayStatics.SpawnEmitterAtLocation` (`self.HitEFX`) _returnvalue)
    (`GameplayStatics.PlaySoundAtLocation` "/Game/Sounds/explosion_large_no_tail_01.explosion_large_no_tail_01" _returnvalue (struct) 1.0 1.0 0.0 null null null)
    (`AISense_Hearing.ReportNoiseEvent` _returnvalue 1.0 (`GameplayStatics.GetPlayerCharacter` 0))
    (`self.K2_DestroyActor`)))

(fn `UserConstructionScript`)