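; Boss enemy that shows its HUD health bar and enters an initial state when a boss-init request fires.
; Health component events update that bar and, at zero health, hide it, stop the boss sound clip and halt the AI controller's movement.
; Helper functions play attack and calm sounds, flag attacking, check the state and gate target following on an accumulated timer.
; BeginPlay also derives health range thresholds from max health.
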(event `self.ReceiveBeginPlay`
  (bind _healthcomponent (`self.HealthComponent`))
  (bind _outactors (`GameplayStatics.GetAllActorsOfClass` "/Script/UnrealStudies.SoundManager"))
  (bind _asbp_sound_manager (cast `/Game/RoomContent/BP_SoundManager` (`|GetArrayItem` _outactors)))
  (set `self.SoundManager` _asbp_sound_manager)
  (bind _outactors_2 (`GameplayStatics.GetAllActorsOfClass` "/Game/GameMode/UnrealStudiesHUD.UnrealStudiesHUD_C"))
  (set `self.HUd` (`|GetArrayItem` _outactors_2))
  (add `self.OnBossInitRequested` (delegate `RequestInit`))
  (`self.InitHealth` _healthcomponent)
  (add `HealthComponent.OnGetDamage` _healthcomponent (delegate `ReduceHealth`))
  (add `HealthComponent.OnHealtToZero` (`self.HealthComponent`) (delegate `FinishBoss`))
  (set `self.InitPos` (`self.K2_GetActorLocation` (`self.initPositioner`))))

(event `ReduceHealth`
  (bind _returnvalue (`HealthComponent.HealthPercentage` (`self.HealthComponent`)))
  (`/Game/GameMode/UnrealStudiesHUD.UpdateHealthBar` (`self.HUd`) _returnvalue))

(event `FinishBoss`
  (`/Game/GameMode/UnrealStudiesHUD.SetVisibilityBossBar` (`self.HUd`) "Hidden")
  (`SoundManager.StopClipBoss` (`self.SoundManager`))
  (bind _asbp_boss_controller (cast `/Game/Enemy/Bp_BossController` (`AIBlueprintHelperLibrary.GetAIController` (`self.GetController`))))
  (`Controller.StopMovement` _asbp_boss_controller))

(event `RequestInit`
  (set `self.ActualState` "NewEnumerator0")
  (`/Game/GameMode/UnrealStudiesHUD.SetVisibilityBossBar` (`self.HUd`) "Visible"))

(event `self.ReceiveTick`
  (params (DeltaSeconds :type "Float (single-precision)")))

(fn `Attack`
  (`SoundManager.PlayClip` (`self.SoundManager`) (`self.SoundAttack`))
  (set `self.isAttacking` true)
  (return))

(fn `CalmStateBossFIght`
  (`SoundManager.PlayClip` (`self.SoundManager`) (`self.SoundCalm`))
  (return))

(fn `CheckIfCalm`
  (returns (NewParam :type Boolean))
  (if (`|EnumEquality` (`self.ActualState`) "NewEnumerator0")
    (return true)
    (else
      (return false))))

(fn `Followtarget`
  (params (NewParam :type "Float (double-precision)"))
  (returns (finishFollowing :type Boolean))
  (if (`self.isAttacking`)
    (bind _output_get (set `self.currentTimer` (+ NewParam (`self.currentTimer`))))
    (bind _returnvalue (>= _output_get 0.0))
    (if _returnvalue
      (return _returnvalue)
      (else
        (return false)))
    (else
      (return false))))

(fn `InitHealth`
  (params (Target :type "HealthComponent Object Reference"))
  (bind _returnvalue (`HealthComponent.GetMaxHealth` Target))
  (set `self.MaxRangeHealth` (`KismetMathLibrary.FTrunc` (* (`KismetMathLibrary.FTrunc` _returnvalue) (`self.HelathMaxPercentage`))))
  (set `self.MinRangeHealth` (`KismetMathLibrary.FTrunc` (* (`KismetMathLibrary.FTrunc` _returnvalue) (`self.HealthLowPercentage`))))
  (return))

(fn `UserConstructionScript`)