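; BP_Rat is an enemy rat character that kills the player on sphere overlap and can explode.
; Every tick it prints its distance to the player, and within the Distance threshold it sets IsNear and disables its movement.
; Explode, not called within this Blueprint, enlarges the sphere to catch the player, plays effect and sound, then destroys the actor.
; The sphere is deactivated at BeginPlay, and its overlap sets BP_PlayableCharacter health to zero.
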(event `self.ReceiveTick`
  (params (DeltaSeconds :type "Float (single-precision)"))
  (`self.CheckDistance`))

(event `self.ReceiveBeginPlay`
  (`ActorComponent.SetActive` (`self.Sphere`) false false))

(event `self.Sphere.OnComponentBeginOverlap`
  (params (OverlappedComponent :type "PrimitiveComponent Object Reference") (OtherActor :type "Actor Object Reference") (OtherComp :type "PrimitiveComponent Object Reference") (OtherBodyIndex :type Integer) (bFromSweep :type Boolean) (SweepResult :type "HitResult Structure (by ref)"))
  (bind _asbp_playable_character (cast `/Game/TPS/BP_PlayableCharacter` OtherActor))
  (`HealthComponent.SetHealthToZero` (`TP_ThirdPersonCharacter.HealthComponent` _asbp_playable_character)))

(fn `CheckDistance`
  (returns (IsNear :type Boolean))
  (bind _returnvalue (`KismetMathLibrary.Vector_Distance` (`self.K2_GetActorLocation`) (`self.K2_GetActorLocation` (`GameplayStatics.GetPlayerPawn` 0))))
  (`KismetSystemLibrary.PrintString` (`KismetStringLibrary.Conv_DoubleToString` _returnvalue))
  (if (< _returnvalue (`self.Distance`))
    (bind _output_get (set `self.isNear` true))
    (`CharacterMovementComponent.DisableMovement` (`self.CharacterMovement`))
    (return _output_get)
    (else
      (return false))))

(fn `Explode`
  (bind _returnvalue (`SceneComponent.K2_GetComponentLocation` (`self.Mesh`)))
  (`SphereComponent.SetSphereRadius` (`self.Sphere`) 400.0 true)
  (`GameplayStatics.SpawnEmitterAtLocation` (`self.Hit EFX`) _returnvalue (struct) (4.0 4.0 4.0))
  (`GameplayStatics.PlaySoundAtLocation` "/Game/Sounds/explosion_large_no_tail_01.explosion_large_no_tail_01" _returnvalue (struct) 1.0 1.0 0.0 null null null)
  (`self.K2_DestroyActor`)
  (return))

(fn `UserConstructionScript`)