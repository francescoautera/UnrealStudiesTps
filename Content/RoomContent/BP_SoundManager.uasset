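; Sound manager for room content that switches music in response to enemy state changes.
; On BeginPlay it caches the enemy list and binds ChangeState to each enemy's OnStateChanged dispatcher, also calling UnbindAllEventsFromOnDestroyed on each loop pass.
; ChangeState passes the new state to PlayMusic and prints a debug string, so music follows events without Tick polling.
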(event `self.ReceiveBeginPlay`
  (bind _returnvalue (`self.GetListEnemies`))
  (bind _output_get (set `self.EnemiesManager` _returnvalue))
  (if (> (`KismetArrayLibrary.Array_Length` _output_get) 0)
    (for _index (range (+ (`KismetArrayLibrary.Array_Length` _output_get) 1))
      (add `EnemyManager.OnStateChanged` (`|GetArrayItem` (`self.EnemiesManager`) _index) (delegate `ChangeState`))
      (clear `Actor.OnDestroyed`))))

(event `ChangeState`
  (params (CurrState :type "EState Enum" :default "Stealth"))
  (`self.PlayMusic` CurrState)
  (`KismetSystemLibrary.PrintString` "Change"))

(fn `UserConstructionScript`)